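; GM_Duel is the game mode for a quick-draw duel between the player and an NPC, run as a phase state machine.
; Tick moves Intro to Wait, then after a random delay enters Draw, broadcasts DrawPhaseStarted and shows the exclamation cue.
; A successful attack defeats the opponent, hides the cue and starts a restart timer.
; Separate functions mark the duel Finished or reset the phase, clock and both duelists.
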(event EventBeginPlay
  (bind _returnvalue (Actor|GetActorOfClass "/Game/BluePrints/BP_Exlamation.BP_Exlamation_C"))
  (Variables|Default|SetExlamationRef _returnvalue)
  (bind _returnvalue_2 (Actor|GetActorOfClass "/Game/BluePrints/BP_Player.BP_Player_C"))
  (Variables|Default|SetPlayer _returnvalue_2)
  (bind _returnvalue_3 (Actor|GetActorOfClass "/Game/BluePrints/BP_NPC.BP_NPC_C"))
  (Variables|Default|SetNPC _returnvalue_3))

(event EventTick
  (params (DeltaSeconds :type Float%20%28single-precision%29))
  (Variables|Default|SetElapsedTime (+ DeltaSeconds (Variables|Default|GetElapsedTime)))
  (switch Utilities|FlowControl|Switch|SwitchonE_Phase (Variables|Default|GetPhase)
    (:NewEnumerator0
      (if (>= (Variables|Default|GetElapsedTime) (Variables|Default|GetRoundStartTime))
        (Variables|Default|SetPhase "NewEnumerator1")
        (Utilities|FlowControl|Delay (Math|Random|RandomFloatinRange (Variables|Default|GetMinDrawDelay) (Variables|Default|GetMaxDrawDelay)))
        (Variables|Default|SetPhase "NewEnumerator2")
        (Default|CallDrawPhaseStarted)
        (Utilities|IsValid (Variables|Default|GetExlamationRef)
          (:Is%20Valid
            (Default|SetVisibility (Variables|Default|GetExlamationRef) true)))))))

(fn ConstructionScript)

(fn SetGameFinished
  (Variables|Default|SetPhase "NewEnumerator3"))

(fn AttackedSuccesfuly
  (params (IsPlayer :type Boolean))
  (if IsPlayer
    (Default|Defeated (Variables|Default|GetNPC))
    (else
      (Default|Defeated (Variables|Default|GetPlayer))))
  (Utilities|IsValid (Variables|Default|GetExlamationRef)
    (:Is%20Valid
      (Default|SetVisibility (Variables|Default|GetExlamationRef) false)
      (Utilities|Time|SetTimerbyEvent (EventDispatchers|CreateEvent :!event Reset) (Variables|Default|GetRestarDelay)))))

(fn Reset
  (Variables|Default|SetPhase "NewEnumerator0")
  (Variables|Default|SetElapsedTime 0.0)
  (Default|Reset (Variables|Default|GetPlayer))
  (Default|Reset (Variables|Default|GetNPC)))